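; Large warehouse door Blueprint that opens when a ThirdPersonCharacter enters its trigger box and closes itself after a delay.
; The overlap snaps DoorWarehouse a quarter turn with an instant relative world rotation, using DoorOpen to prevent repeat opening.
; Tick polls DoorOpen and runs a Delay of CloseDelay before rotating back, regardless of whether the character is still inside.
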(event `self.ReceiveTick`
  (params (DeltaSeconds :type "Float (single-precision)"))
  (if (`self.doorOpen`)
    (`KismetSystemLibrary.Delay` (`self.closeDelay`))
    (`SceneComponent.K2_AddWorldRotation` (`self.doorWarehouse`) (struct :`Yaw` -90.0) false false)
    (set `self.doorOpen` false)))

(event `self.EnterBox.OnComponentBeginOverlap`
  (params (OverlappedComponent :type "PrimitiveComponent Object Reference") (OtherActor :type "Actor Object Reference") (OtherComp :type "PrimitiveComponent Object Reference") (OtherBodyIndex :type Integer) (bFromSweep :type Boolean) (SweepResult :type "HitResult Structure (by ref)"))
  (cast `/Game/ThirdPersonBP/Blueprints/ThirdPersonCharacter` OtherActor)
  (if (not (`self.doorOpen`))
    (`SceneComponent.K2_AddWorldRotation` (`self.doorWarehouse`) (struct :`Yaw` 90.0) false false)
    (set `self.doorOpen` true)))

(fn `UserConstructionScript`)