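; BP_Door is a door that opens when a ThirdPersonCharacter enters its trigger box and closes after a three-second delay.
; The box overlap sets a DoorIsOpen flag, ignoring further overlaps until it resets.
; Tick reads the flag every frame and snaps the Door01e component between an open location with fixed rotation and its original location, without interpolation.
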(event `self.ReceiveBeginPlay`)

(event `self.ReceiveTick`
  (params (DeltaSeconds :type "Float (single-precision)"))
  ;[1 1 1] Open Door (Archive)
  (if (`self.doorIsOpen`)
    (`SceneComponent.K2_SetWorldLocationAndRotation` (`self.door01e`) (`self.newLocation`) (struct :`Yaw` 90.0) false false)
    (else
      (`SceneComponent.K2_SetWorldLocationAndRotation` :`self` (`self.door01e`) :`NewLocation` (`self.originalLocation`)))))

(event `self.Box.OnComponentBeginOverlap`
  (params (OverlappedComponent :type "PrimitiveComponent Object Reference") (OtherActor :type "Actor Object Reference") (OtherComp :type "PrimitiveComponent Object Reference") (OtherBodyIndex :type Integer) (bFromSweep :type Boolean) (SweepResult :type "HitResult Structure (by ref)"))
  ;[1 1 1] Open Door (Archive)
  (cast `/Game/ThirdPersonBP/Blueprints/ThirdPersonCharacter` OtherActor)
  (if (not (`self.doorIsOpen`))
    (set `self.doorIsOpen` true)
    (`KismetSystemLibrary.Delay` 3.0)
    (set `self.doorIsOpen` false)))

(fn `UserConstructionScript`)